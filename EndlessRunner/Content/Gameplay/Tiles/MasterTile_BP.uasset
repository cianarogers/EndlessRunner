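; Base floor tile for a three-lane endless runner that populates itself with obstacles and pickups.
; On BeginPlay, each lane gets a chained random roll for a log obstacle, turkey, meat or magnet, re-rolled at each check, so a lane can stay empty.
; When the character overlaps the Box, it has the GameMode spawn another tile, adds multiplied points, raises clamped walk speed, then destroys itself after a short delay.
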(event `self.Box.OnComponentBeginOverlap`
  (params (OverlappedComponent :type "PrimitiveComponent Object Reference") (OtherActor :type "Actor Object Reference") (OtherComp :type "PrimitiveComponent Object Reference") (OtherBodyIndex :type Integer) (bFromSweep :type Boolean) (SweepResult :type "HitResult Structure (by ref)"))
  ;[1 1 1] Adds 2 points for every tile run over and increases running speed over time
  (bind _asthird_person_character (cast `/Game/Gameplay/Player/ThirdPersonCharacter` OtherActor))
  (bind _asthird_person_game_mode (cast `/Game/Gameplay/GameMode/ThirdPersonGameMode` (`GameplayStatics.GetGameMode`)))
  (`/Game/Gameplay/GameMode/ThirdPersonGameMode.SpawnTile` _asthird_person_game_mode)
  (set `/Game/Gameplay/GameMode/ThirdPersonGameMode.CurrentPoints` (+ (* 1 (`/Game/Gameplay/GameMode/ThirdPersonGameMode.PointsMultiplier` _asthird_person_game_mode)) (`/Game/Gameplay/GameMode/ThirdPersonGameMode.CurrentPoints` _asthird_person_game_mode)) _asthird_person_game_mode)
  (bind _charactermovement (`Character.CharacterMovement` _asthird_person_character))
  (set `CharacterMovementComponent.MaxWalkSpeed` (`KismetMathLibrary.FClamp` (* (`CharacterMovementComponent.MaxWalkSpeed` _charactermovement) 1.01) 600.0 2000.0) _charactermovement)
  (`KismetSystemLibrary.Delay` 0.5)
  (`self.K2_DestroyActor`))

(event `self.ReceiveBeginPlay`
  (`self.SpawnObstacles`))

(fn `SpawnObstacle`
  (params (self2 :type "SceneComponent Object Reference"))
  (bind _returnvalue (`SceneComponent.K2_GetComponentToWorld` self2))
  (bind _returnvalue_2 (`KismetMathLibrary.RandomFloatInRange` 0.0 1.0))
  (if (`KismetMathLibrary.InRange_FloatFloat` _returnvalue_2 0.0 0.4)
    (`|SpawnActorFromClass` "/Game/Gameplay/Obstacles/Obstacle_LogPile.Obstacle_LogPile_C" _returnvalue "Undefined" "OverrideRootScale" null null)
    (elif (`KismetMathLibrary.InRange_FloatFloat` _returnvalue_2 0.4 0.5)
      (`|SpawnActorFromClass` "/Game/Gameplay/Obstacles/Obstacle_LogLarge.Obstacle_LogLarge_C" _returnvalue "Undefined" "OverrideRootScale" null null)
      (elif (`KismetMathLibrary.InRange_FloatFloat` _returnvalue_2 0.5 0.7)
        (`|SpawnActorFromClass` "/Game/Gameplay/Pickups/Pickup_Turkey.Pickup_Turkey_C" _returnvalue "Undefined" "OverrideRootScale" null null)
        (elif (`KismetMathLibrary.InRange_FloatFloat` _returnvalue_2 0.7 0.9)
          (`|SpawnActorFromClass` "/Game/Gameplay/Pickups/Pickup_Meat.Pickup_Meat_C" _returnvalue "Undefined" "OverrideRootScale" null null)
          (elif (`KismetMathLibrary.InRange_FloatFloat` _returnvalue_2 0.9)
            (`|SpawnActorFromClass` "/Game/Gameplay/Pickups/Pickup_Magnet.Pickup_Magnet_C" _returnvalue "Undefined" "OverrideRootScale" null null)))))))

(fn `SpawnObstacles`
  ;[1 1 1] Lane 0
  (`self.SpawnObstacle` (`self.Lane`))
  (`self.SpawnObstacle` (`self.Lane1`))
  (`self.SpawnObstacle` (`self.Lane2`)))

(fn `UserConstructionScript`)